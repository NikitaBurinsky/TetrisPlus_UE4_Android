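; Player pawn for a 3D Tetris game that owns the main, pause and gameplay widgets, music and score presentation.
; BeginPlay builds the widgets, creates dynamic materials on mesh arrays and starts music.
; Tetris events refresh the next-figure viewer and 3D text stats with a sound and timeline camera bump, or play a line-clear sound.
; Start and pause handlers toggle the 3D touch interface, menus, cursor and input mode.
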(event `self.ReceiveBeginPlay`
  (bind _returnvalue (`GameplayStatics.GetPlayerController` 0))
  (bind _returnvalue_2 (`|CreateWidget` "/Game/Menu/GP_Widget/GP_Widget_Mobile.GP_Widget_Mobile_C" (`GameplayStatics.GetPlayerController` 0)))
  (bind _output_get (set `self.GP Widget` _returnvalue_2))
  (`UserWidget.AddToViewport` _output_get 0)
  (`Widget.SetVisibility` _output_get "Hidden")
  (bind _returnvalue_3 (`|CreateWidget` "/Game/Menu/PauseMenu/Pause_Menu.Pause_Menu_C" (`GameplayStatics.GetPlayerController` 0)))
  (bind _output_get_2 (set `self.Pause Menu` _returnvalue_3))
  (`UserWidget.AddToViewport` _output_get_2 0)
  (`Widget.SetVisibility` _output_get_2 "Hidden")
  (bind _returnvalue_4 (`|CreateWidget` "/Game/Menu/MainMenu/Main_Menu_Mobile.Main_Menu_Mobile_C" _returnvalue))
  (bind _output_get_3 (set `self.MainMenu` _returnvalue_4))
  (`UserWidget.AddToViewport` _output_get_3 0)
  (`WidgetBlueprintLibrary.SetInputMode_GameAndUIEx` _returnvalue _output_get_3 "DoNotLock" false)
  (set `PlayerController.bShowMouseCursor` true _returnvalue)
  (set `self.Was` true)
  (`|ExecutionSequence`
    (:`then_0`
      (for _array_element _
        (`PrimitiveComponent.CreateDynamicMaterialInstance` (`StaticMeshActor.StaticMeshComponent` _array_element) 0 (`StaticMesh.GetMaterial` (`StaticMeshComponent.StaticMesh` (`StaticMeshActor.StaticMeshComponent` _array_element)) 0) "BaseColor")))
    (:`then_1`
      (`self.Play Music`))))

(event `self.OnTetrisScoreUpdated`
  (if (`self.Was`)
    (bind _returnvalue (`Tetris_Core.GetPublicUIData` (`self.Tetris`)))
    (`Tetris_NF_Viewer.UpdateNextFigureViewer` (`self.Tetris_NF_Viewer`) (`.NextFigure` (break `AllExtraValues` _returnvalue)))
    ;[1 1 1] test
    (`self.Upgate 3D Scores` _returnvalue)
    (`GameplayStatics.SpawnSound2D` "/Game/Sound/1.1" 1.0 1.0 0.0 null)
    (set `self.Relative Location` (`SceneComponent.RelativeLocation` (`self.Camera`)))
    (bind (_direction _z_offset) (`Timeline|Timeline_0` :!via `PlayFromStart`)
      (:`Update`
        (`SceneComponent.K2_AddRelativeLocation` (`self.Camera`) (`KismetMathLibrary.MakeVector` 0.0 0.0 _z_offset) false false))
      (:`Finished`
        (`SceneComponent.K2_SetRelativeLocation` (`self.Camera`) (`self.Relative Location`) false false)))))

(event `self.OnGamePaused`
  (bind _returnvalue (`GameplayStatics.GetPlayerController` 0))
  (bind _pause_menu (`self.Pause Menu`))
  (`/Game/BP_Touch3DImplementation.Deactivate Interface` (`self.3D Touch Interface`))
  (`Widget.SetVisibility` _pause_menu "Visible")
  (`WidgetBlueprintLibrary.SetInputMode_GameAndUIEx` _returnvalue _pause_menu "LockInFullscreen" false)
  (set `PlayerController.bShowMouseCursor` true _returnvalue))

(event `self.OnGameUnPaused`
  (bind _returnvalue (`GameplayStatics.GetPlayerController` 0))
  (`/Game/BP_Touch3DImplementation.Activate Interface` (`self.3D Touch Interface`))
  (`Widget.SetVisibility` (`self.Pause Menu`) "Hidden")
  (`WidgetBlueprintLibrary.SetInputMode_GameAndUIEx` _returnvalue null)
  (set `PlayerController.bShowMouseCursor` false _returnvalue))

(event `self.OnLineDestroyed`
  (`GameplayStatics.PlaySound2D` "/Game/Sound/2_2.2_2" 1.0 1.0 0.0 null null false))

(fn `AddScoreVibration`
  (`PlayerController.K2_ClientPlayForceFeedback` (`GameplayStatics.GetPlayerController` 0) "/Game/VibrationAssets/AddScore_FF.AddScore_FF" "v" false false false)
  (return))

(fn `Change Pause To Menu`
  (`Tetris_Core.EndGameBP` (`self.Tetris`))
  (`Widget.SetVisibility` (`self.Pause Menu`) "Collapsed")
  (`Widget.SetVisibility` (`self.MainMenu`) "Visible")
  (`WidgetBlueprintLibrary.SetInputMode_GameAndUIEx` (`GameplayStatics.GetPlayerController` 0) (`self.MainMenu`) "DoNotLock" false))

(fn `UI_StartTetrisGame`
  (bind _returnvalue (`GameplayStatics.GetPlayerController` 0))
  (`/Game/BP_Touch3DImplementation.Activate Interface` (`self.3D Touch Interface`))
  (`Widget.SetVisibility` (`self.MainMenu`) "Hidden")
  (`WidgetBlueprintLibrary.SetInputMode_GameOnly` _returnvalue)
  (set `PlayerController.bShowMouseCursor` false _returnvalue))

(fn `UserConstructionScript`)