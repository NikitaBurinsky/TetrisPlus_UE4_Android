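; Actor providing 3D touch buttons that control the falling figure (move, rotate, drop) along with pause and restart.
; On BeginPlay it caches BP_PlayerPawn and enables touch-over events, then component touch events call the pawn's matching functions.
; Helpers shift buttons along Y as press feedback; touch leave counts as release, while menu and restart pop back after a delay.
; ActivateInterface and DeactivateInterface toggle visibility of the movement buttons.
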(event `self.ReceiveBeginPlay`
  (bind _asbp_player_pawn (cast `/Game/BP_PlayerPawn` (`GameplayStatics.GetPlayerPawn` 0)))
  (set `self.As BP Player Pawn` _asbp_player_pawn)
  (set `PlayerController.bEnableTouchOverEvents` true (`GameplayStatics.GetPlayerController` 0)))

(event `Activate Interface`
  ;[1 1 1] Activate/ Deactivate
  (`SceneComponent.SetVisibility` (`self.Left`) true false)
  (`SceneComponent.SetVisibility` (`self.Right`) true false)
  (`SceneComponent.SetVisibility` (`self. Super Down`) true false)
  (`SceneComponent.SetVisibility` (`self.Down`) true false)
  (`SceneComponent.SetVisibility` (`self.Rotate`) true false)
  (set `self.IsActivated?` true))

(event `Deactivate Interface`
  ;[1 1 1] Activate/ Deactivate
  (`SceneComponent.SetVisibility` (`self.Left`) false false)
  (`SceneComponent.SetVisibility` (`self.Right`) false false)
  (`SceneComponent.SetVisibility` (`self. Super Down`) false false)
  (`SceneComponent.SetVisibility` (`self.Down`) false false)
  (`SceneComponent.SetVisibility` (`self.Rotate`) false false)
  (set `self.IsActivated?` false))

(event `self.Rotate.OnInputTouchBegin`
  (params (FingerIndex :type "ETouchIndex Enum" :default "Touch1") (TouchedComponent :type "PrimitiveComponent Object Reference"))
  ;[1 1 1] Touch Rotate
  (`PlayerPawn.RotateFigure` (`self.As BP Player Pawn`))
  (`self.Make Button Down` (`self.Rotate`)))

(event `self.Rotate.OnInputTouchEnd`
  (params (FingerIndex :type "ETouchIndex Enum" :default "Touch1") (TouchedComponent :type "PrimitiveComponent Object Reference"))
  ;[1 1 1] Touch Rotate
  (`self.Make Button Up` (`self.Rotate`) :!label _label))

(event `self.MenuCollision.OnInputTouchBegin`
  (params (FingerIndex :type "ETouchIndex Enum" :default "Touch1") (TouchedComponent :type "PrimitiveComponent Object Reference"))
  (bind _menu (`self.Menu`))
  ;[1 0.2344 0.2344] Menu Touch
  (`self.Make SubButton Down` _menu)
  (`|ExecutionSequence`
    (:`then_0`
      (`PlayerPawn.GamePauseButtonPressed` (`self.As BP Player Pawn`))
      (`GameplayStatics.PlaySound2D` "/Game/Sound/s.s" 1.0 1.0 0.0 null null))
    (:`then_1`
      (`KismetSystemLibrary.Delay` 0.2)
      (`self.Make SubButton Up` _menu))))

(event `self.Rotate.OnInputTouchLeave`
  (params (FingerIndex :type "ETouchIndex Enum" :default "Touch1") (TouchedComponent :type "PrimitiveComponent Object Reference"))
  ;[1 1 1] Touch Rotate
  (goto _label))

(event `self.Right.OnInputTouchBegin`
  (params (FingerIndex :type "ETouchIndex Enum" :default "Touch1") (TouchedComponent :type "PrimitiveComponent Object Reference"))
  ;[1 1 1] Right Touch
  (`PlayerPawn.MoveFigureRight` (`self.As BP Player Pawn`))
  (`self.Make Button Down` (`self.Right`)))

(event `self.RestartCollison.OnInputTouchBegin`
  (params (FingerIndex :type "ETouchIndex Enum" :default "Touch1") (TouchedComponent :type "PrimitiveComponent Object Reference"))
  (bind _restart (`self.Restart`))
  ;[1 0.2344 0.2344] Restart Touch
  (`self.Make SubButton Down` _restart)
  (`|ExecutionSequence`
    (:`then_0`
      (`/Engine/EditorBlueprintResources/StandardMacros.DoOnce` false :!label _label_2
        (:`Completed`
          (`PlayerPawn.TEST_RESTART` (`self.As BP Player Pawn`))
          (`GameplayStatics.PlaySound2D` "/Game/Sound/restart.restart" 1.0 1.0 0.0 null null)
          (`KismetSystemLibrary.Delay` 1.0)
          (goto _label_2 :!via `Reset`))))
    (:`then_1`
      (`KismetSystemLibrary.Delay` 0.2)
      (`self.Make SubButton Up` _restart))))

(event `self.Right.OnInputTouchEnd`
  (params (FingerIndex :type "ETouchIndex Enum" :default "Touch1") (TouchedComponent :type "PrimitiveComponent Object Reference"))
  ;[1 1 1] Right Touch
  (`PlayerPawn.MoveFigureRight_Released` (`self.As BP Player Pawn`) :!label _label_3)
  (`self.Make Button Up` (`self.Right`)))

(event `self.Right.OnInputTouchLeave`
  (params (FingerIndex :type "ETouchIndex Enum" :default "Touch1") (TouchedComponent :type "PrimitiveComponent Object Reference"))
  ;[1 1 1] Right Touch
  (goto _label_3))

(event `self. Super Down.OnInputTouchBegin`
  (params (FingerIndex :type "ETouchIndex Enum" :default "Touch1") (TouchedComponent :type "PrimitiveComponent Object Reference"))
  ;[1 1 1] Super Down Touch
  (`PlayerPawn.MoveSuperDown` (`self.As BP Player Pawn`))
  (`self.Make Button Down` (`self. Super Down`)))

(event `self. Super Down.OnInputTouchEnd`
  (params (FingerIndex :type "ETouchIndex Enum" :default "Touch1") (TouchedComponent :type "PrimitiveComponent Object Reference"))
  ;[1 1 1] Super Down Touch
  (`self.Make Button Up` (`self. Super Down`) :!label _label_4))

(event `self. Super Down.OnInputTouchLeave`
  (params (FingerIndex :type "ETouchIndex Enum" :default "Touch1") (TouchedComponent :type "PrimitiveComponent Object Reference"))
  ;[1 1 1] Super Down Touch
  (goto _label_4))

(event `self.Down.OnInputTouchBegin`
  (params (FingerIndex :type "ETouchIndex Enum" :default "Touch1") (TouchedComponent :type "PrimitiveComponent Object Reference"))
  ;[1 1 1] Down Touch
  (`PlayerPawn.MoveDownButtonPressed` (`self.As BP Player Pawn`))
  (`self.Make Button Down` (`self.Down`)))

(event `self.Down.OnInputTouchEnd`
  (params (FingerIndex :type "ETouchIndex Enum" :default "Touch1") (TouchedComponent :type "PrimitiveComponent Object Reference"))
  ;[1 1 1] Down Touch
  (`PlayerPawn.MoveDownButtonReleased` (`self.As BP Player Pawn`) :!label _label_5)
  (`self.Make Button Up` (`self.Down`)))

(event `self.Down.OnInputTouchLeave`
  (params (FingerIndex :type "ETouchIndex Enum" :default "Touch1") (TouchedComponent :type "PrimitiveComponent Object Reference"))
  ;[1 1 1] Down Touch
  (goto _label_5))

(event `self.Left.OnInputTouchBegin`
  (params (FingerIndex :type "ETouchIndex Enum" :default "Touch1") (TouchedComponent :type "PrimitiveComponent Object Reference"))
  ;[1 1 1] Left Touch
  (`PlayerPawn.MoveFigureLeft` (`self.As BP Player Pawn`))
  (`self.Make Button Down` (`self.Left`)))

(event `self.Left.OnInputTouchEnd`
  (params (FingerIndex :type "ETouchIndex Enum" :default "Touch1") (TouchedComponent :type "PrimitiveComponent Object Reference"))
  ;[1 1 1] Left Touch
  (`PlayerPawn.MoveFigureLeft_Released` (`self.As BP Player Pawn`) :!label _label_6)
  (`self.Make Button Up` (`self.Left`)))

(event `self.Left.OnInputTouchLeave`
  (params (FingerIndex :type "ETouchIndex Enum" :default "Touch1") (TouchedComponent :type "PrimitiveComponent Object Reference"))
  ;[1 1 1] Left Touch
  (goto _label_6))

(fn `Make Button Down`
  (params (Button :type "StaticMeshComponent Object Reference"))
  (bind (_relativelocation_x _relativelocation_y _relativelocation_z) (`KismetMathLibrary.BreakVector` (`SceneComponent.RelativeLocation` Button)))
  (`SceneComponent.K2_SetRelativeLocation` Button (`KismetMathLibrary.MakeVector` _relativelocation_x (`self.Buttons Down Lenght`) _relativelocation_z) false false))

(fn `Make Button Up`
  (params (Target :type "SceneComponent Object Reference"))
  (bind (_relativelocation_x _relativelocation_y _relativelocation_z) (`KismetMathLibrary.BreakVector` (`SceneComponent.RelativeLocation` Target)))
  (`SceneComponent.K2_SetRelativeLocation` Target (`KismetMathLibrary.MakeVector` _relativelocation_x 0.0 _relativelocation_z) false false))

(fn `Make SubButton Down`
  (params (Button :type "StaticMeshComponent Object Reference"))
  (`SceneComponent.K2_AddRelativeLocation` Button (`KismetMathLibrary.MakeVector` 0.0 (* (`self.SubButtonsDownLenght`) -1.0)) false false)
  (return))

(fn `Make SubButton Up`
  (params (Target :type "SceneComponent Object Reference"))
  (`SceneComponent.K2_AddRelativeLocation` Target (`KismetMathLibrary.MakeVector` 0.0 (`self.SubButtonsDownLenght`)) false false))

(fn `UserConstructionScript`)